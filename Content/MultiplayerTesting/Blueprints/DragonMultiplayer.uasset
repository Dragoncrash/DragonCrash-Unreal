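; Multiplayer player dragon with toggleable hover and flight modes, a timed fire-breath projectile and server-authoritative ramming that destroys other dragons at crash speed.
; Tick runs the active mode: hover strafes and ascends, while flight steers by controller rotation and eases speed toward normal or boosted limits.
; Boosting drains energy, which recharges after a delay; exhaustion blocks boosting until mostly refilled.
; Construction converts speeds and accelerations into MaxFlySpeed fractions for movement-input scaling.
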(event Custom|BreathAttack1
  ;[1 1 1] Breath Attack 1
  (CallFunction|FireBreath1))

(event EventTick
  (params (DeltaSeconds :type Float%20%28single-precision%29))
  (Utilities|FlowControl|Sequence
    (:then_0
      ;[1 1 1] Flight Mode Branch
      (if (Variables|Default|GetIsFlightMode)
        (CallFunction|FlightModeTick DeltaSeconds)
        (else
          (CallFunction|HoverModeTick DeltaSeconds))))
    (:then_1
      ;[1 1 1] Energy Regeneration Logic
      (if (<= (- (Variables|Default|GetEnergyTimer) DeltaSeconds) 0.0)
        (Variables|Default|SetEnergy (Math|Float|Min(Float) (+ (Variables|Default|GetEnergy) (* (Variables|Energy|GetEnergyRechargeRate) DeltaSeconds)) (Variables|Energy|GetEnergyMax)))
        (else
          (Variables|Default|SetEnergyTimer (- (Variables|Default|GetEnergyTimer) DeltaSeconds)))))
    (:then_2
      ;[1 1 1] Exhaustion Logic
      (if (>= (Variables|Default|GetEnergy) (* (Variables|Energy|GetEnergyMax) 0.8))
        (Variables|Default|SetIsExhausted false)))
    (:then_3
      ;[1 1 1] Breath Attack Cooldown Logic
      (if (> (Variables|Default|GetBreathTimer1) 0.0)
        (Variables|Default|SetBreathTimer1 (- (Variables|Default|GetBreathTimer1) DeltaSeconds))))))

(event Collision|EventHit
  (params (MyComp :type Primitive%20Component%20Object%20Reference) (Other :type Actor%20Object%20Reference) (OtherComp :type Primitive%20Component%20Object%20Reference) (bSelfMoved :type Boolean) (HitLocation :type Vector :default "0, 0, 0") (HitNormal :type Vector :default "0, 0, 0") (NormalImpulse :type Vector :default "0, 0, 0") (Hit :type Hit%20Result%20Structure%20%28by%20ref%29))
  (Networking|SwitchHasAuthority
    (:Authority
      (bind _asdragon_multiplayer (Utilities|Casting|CastToDragonMultiplayer Other))
      (if (>= (Math|Vector|VectorLength (Transformation|GetVelocity)) (Variables|DragonCrashing|GetDragonCrashingSpeed))
        (Actor|DestroyActor _asdragon_multiplayer)))))

(event Input|ActionEvents|InputActionBreath1
  (params (Key :type Key%20Structure :default "AnyKey"))
  ;[1 1 1] Breath Attack 1
  (:Pressed
    (CallFunction|BreathAttack1)))

(event Input|ActionEvents|InputActionChangeMode
  (params (Key :type Key%20Structure :default "AnyKey"))
  ;[1 1 1] Flight Mode Switching
  (:Released
    (Variables|Default|SetIsFlightMode (not (Variables|Default|GetIsFlightMode)))))

(event Input|ActionEvents|InputActionDragonCrash
  (params (Key :type Key%20Structure :default "AnyKey"))
  ;[1 1 1] Boost Input Logic
  (:Pressed
    (Variables|Default|SetIsFlightMode true)
    (Variables|Default|SetIsBoosting true))
  (:Released
    (Variables|Default|SetIsBoosting false)))

(fn ConstructionScript
  ;[1 1 1] Max Out Energy
  (Variables|Default|SetEnergy (Variables|Energy|GetEnergyMax))
  ;[1 1 1] Convert Accelerations and Speeds to Max Fly Speed Scalars
  (Variables|HoverMode|SetHoverForwardSpeed (Utilities|SpeedtoMaxFlySpeedScalar (Variables|HoverMode|GetHoverForwardSpeed)))
  (Variables|HoverMode|SetHoverAscendSpeed (Utilities|SpeedtoMaxFlySpeedScalar (Variables|HoverMode|GetHoverAscendSpeed)))
  (Variables|FlightMode|SetFlightAcceleration (Utilities|SpeedtoMaxFlySpeedScalar (Variables|FlightMode|GetFlightAcceleration)))
  (Variables|FlightMode|SetFlightMaxSpeed (Utilities|SpeedtoMaxFlySpeedScalar (Variables|FlightMode|GetFlightMaxSpeed)))
  (Variables|Boosting|SetAccelerationBoosting (Utilities|SpeedtoMaxFlySpeedScalar (Variables|Boosting|GetAccelerationBoosting)))
  (Variables|Boosting|SetMaxSpeedBoosting (Utilities|SpeedtoMaxFlySpeedScalar (Variables|Boosting|GetMaxSpeedBoosting))))

(fn HoverModeTick
  (params (Delta%20Seconds :type Float%20%28single-precision%29))
  (Utilities|FlowControl|Sequence
    (:then_0
      ;[1 1 1] Apply Pitch Input
      (Pawn|Input|AddControllerPitchInput (Input|AxisValues|GetLookUp)))
    (:then_1
      ;[1 1 1] Apply Yaw Input
      (Pawn|Input|AddControllerYawInput (Input|AxisValues|GetTurn)))
    (:then_2
      ;[1 1 1] Right/Left Movement
      (Pawn|Input|AddMovementInput (Math|Vector|GetRightVector (Variables|Default|GetSpringArm)) (* (Input|AxisValues|GetMoveRight) (Variables|HoverMode|GetHoverForwardSpeed)) false))
    (:then_3
      ;[1 1 1] Forward/Backward Movement
      (Pawn|Input|AddMovementInput (Math|Vector|GetForwardVector (Variables|Default|GetSpringArm)) (* (Input|AxisValues|GetMoveForward) (Variables|HoverMode|GetHoverForwardSpeed)) false))
    (:then_4
      ;[1 1 1] Ascend/Descend Movement
      (Pawn|Input|AddMovementInput (Math|Vector|GetUpVector (Variables|Default|GetDragon_static)) (* (Input|AxisValues|GetAscend) (Variables|HoverMode|GetHoverAscendSpeed)) false))))

(fn FlightModeTick
  (params (Delta%20Seconds :type Float%20%28single-precision%29))
  (bind _returnvalue (Transformation|GetVelocity))
  (bind _returnvalue_2 (Math|Vector|VectorLength _returnvalue))
  (bind _scale (Utilities|SpeedtoMaxFlySpeedScalar _returnvalue_2))
  (Utilities|FlowControl|Sequence
    (:then_0
      ;[1 1 1] Apply Pitch Input
      (Pawn|Input|AddControllerPitchInput (Input|AxisValues|GetMoveForward)))
    (:then_1
      ;[1 1 1] Apply Yaw Input
      (Pawn|Input|AddControllerYawInput (Input|AxisValues|GetMoveRight)))
    (:then_2
      ;[1 1 1] Boosting Logic
      (LocalVariables|SetCanBoost false)
      (if (and (Variables|Default|GetIsBoosting) (not (Variables|Default|GetIsExhausted)))
        (if (> (Variables|Default|GetEnergy) 0.0)
          (LocalVariables|SetCanBoost true)
          (Variables|Default|SetEnergy (- (Variables|Default|GetEnergy) Delta%20Seconds))
          (Variables|Default|SetEnergyTimer (Variables|Energy|GetEnergyRechargeDelay))
          (else
            (Variables|Default|SetIsExhausted true)))))
    (:then_3
      ;[1 1 1] Determine Desired Acceleration and Speed
      (if (LocalVariables|GetCanBoost)
        (LocalVariables|SetDesiredSpeed (Variables|Boosting|GetMaxSpeedBoosting))
        (LocalVariables|SetDesiredAcceleration (Variables|Boosting|GetAccelerationBoosting))
        (else
          (LocalVariables|SetDesiredSpeed (Variables|FlightMode|GetFlightMaxSpeed))
          (LocalVariables|SetDesiredAcceleration (Variables|FlightMode|GetFlightAcceleration)))))
    (:then_4
      ;[1 1 1] Movement
      (Pawn|Input|AddMovementInput (Math|Vector|RotateVectorAroundAxis (Math|Vector|GetRightVector (Variables|Default|GetDragon_static)) (* (Input|AxisValues|GetAscend) (Variables|FlightMode|GetFlightAscendAngle)) (Math|Vector|GetForwardVector (Variables|Default|GetDragon_static))) (+ _scale (Math|Float|Min(Float) (- (LocalVariables|GetDesiredSpeed) _scale) (* Delta%20Seconds (LocalVariables|GetDesiredAcceleration)))) false))))

(fn FireBreath1
  (if (<= (Variables|Default|GetBreathTimer1) 0.0)
    (Variables|Default|SetBreathTimer1 (Variables|BreathAttacks|GetBreathCooldown1))
    (bind _returnvalue (Game|SpawnActorfromClass (Variables|BreathAttacks|GetBreathProjectile1) (Transformation|GetWorldTransform (Variables|Default|GetProjectile_SpawnLocation)) "AdjustIfPossibleButAlwaysSpawn" 0 0))
    (Variables|/Game/MultiplayerTesting/Blueprints/ProjectileBaseMultiplayer.ProjectileBaseMultiplayer_C|SetDirection _returnvalue (Math|Vector|GetForwardVector (Variables|Default|GetSpringArm)))))